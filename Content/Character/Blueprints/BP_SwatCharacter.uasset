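; Player character Blueprint for a SWAT character, using Enhanced Input for movement, camera look, jump, sprint and a weapon-equip toggle.
; BeginPlay adds the combat mapping context and orients rotation to movement.
; Sprint changes a clamped WalkSpeed target, which MaxWalkSpeed eases toward through FInterpTo only while move input fires.
; The equip FlipFlop sets a weapon flag and switches between movement-oriented and controller-yaw rotation.
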(event Input|EnhancedActionEvents|EnhancedInputActionIA_Jump
  (params (ActionValue :type Boolean) (ElapsedSeconds :type Float%20%28double-precision%29) (TriggeredSeconds :type Float%20%28double-precision%29) (InputAction :type Input%20Action%20Object%20Reference :default "/Game/Character/Actions/Inputs/IA_Jump.IA_Jump"))
  ;[0.8284 1 0.02812] Pular
  (:Triggered
    (Character|Jump))
  (:Completed
    (Character|StopJumping)))

(event Input|EnhancedActionEvents|EnhancedInputActionIA_Look
  (params (ActionValue :type Vector%202D%20Structure) (ElapsedSeconds :type Float%20%28double-precision%29) (TriggeredSeconds :type Float%20%28double-precision%29) (InputAction :type Input%20Action%20Object%20Reference :default "/Game/Character/Actions/Inputs/IA_Look.IA_Look"))
  ;[0.027 0.3902 1] Camera
  (Pawn|Input|AddControllerYawInput (.x ActionValue))
  (Pawn|Input|AddControllerPitchInput (.y ActionValue)))

(event Input|EnhancedActionEvents|EnhancedInputActionIA_Move
  (params (ActionValue :type Vector%202D%20Structure) (ElapsedSeconds :type Float%20%28double-precision%29) (TriggeredSeconds :type Float%20%28double-precision%29) (InputAction :type Input%20Action%20Object%20Reference :default "/Game/Character/Actions/Inputs/IA_Move.IA_Move"))
  (bind _returnvalue (Pawn|GetControlRotation :!class /Script/Engine.Pawn))
  ;[1 0 0] Movimento de caminhar
  ;;[1 1 1] Movimento Esquerda/Direita
  (CallFunction|FInterpWlakSpeed)
  (Pawn|Input|AddMovementInput (Math|Vector|GetRightVector (Math|Rotator|MakeRotator (.roll _returnvalue) 0.0 (.yaw _returnvalue))) (.x ActionValue) false)
  ;;[1 1 1] Movimento Frente/Trás
  (CallFunction|FInterpWlakSpeed)
  (Pawn|Input|AddMovementInput (Math|Vector|GetForwardVector (Math|Rotator|MakeRotator 0.0 0.0 (.yaw (Pawn|GetControlRotation :!class /Script/Engine.Pawn)))) (.y ActionValue) false))

(event Input|EnhancedActionEvents|EnhancedInputActionIA_Sprint
  (params (ActionValue :type Boolean) (ElapsedSeconds :type Float%20%28double-precision%29) (TriggeredSeconds :type Float%20%28double-precision%29) (InputAction :type Input%20Action%20Object%20Reference :default "/Game/Character/Actions/Inputs/IA_Sprint.IA_Sprint"))
  ;[1 0.1674 0.6073] Botão de sprint
  (:Started
    (Variables|Default|Setsprint true)
    (Variables|Default|SetWalkSpeed (Math|Float|Clamp(Float) (* (Variables|Default|GetWalkSpeed) 3.0) 3e+02 6e+02)))
  (:Completed
    (Variables|Default|Setsprint false)
    (Variables|Default|SetWalkSpeed (Math|Float|Clamp(Float) (* (Variables|Default|GetWalkSpeed) 0.5) 3e+02 3e+02))))

(event Input|EnhancedActionEvents|EnhancedInputActionIA_EquipeWeapon
  (params (ActionValue :type Boolean) (ElapsedSeconds :type Float%20%28double-precision%29) (TriggeredSeconds :type Float%20%28double-precision%29) (InputAction :type Input%20Action%20Object%20Reference :default "/Game/Character/Actions/Inputs/IA_EquipeWeapon.IA_EquipeWeapon"))
  (bind _charactermovement (Variables|Character|GetCharacterMovement))
  ;[0.1393 1 0.08227] Equipar Jogador
  (Utilities|FlowControl|FlipFlop
    (:A
      (Variables|Default|SetEquipWeaponBPSwat true)
      (Variables|/Script/Engine.CharacterMovementComponent|SetbOrientRotationToMovement _charactermovement false)
      (Variables|Default|SetbUseControllerRotationYaw true))
    (:B
      (Variables|Default|SetEquipWeaponBPSwat false)
      (Variables|/Script/Engine.CharacterMovementComponent|SetbOrientRotationToMovement _charactermovement true)
      (Variables|Default|SetbUseControllerRotationYaw false))))

(event EventBeginPlay
  ;[0.1067 1 0.5288] Mapeando Controle antes do Jogo começar
  (Variables|/Script/Engine.CharacterMovementComponent|SetbOrientRotationToMovement (Variables|Character|GetCharacterMovement) true)
  (Variables|Default|SetbUseControllerRotationYaw false)
  (bind _asplayer_controller (Utilities|Casting|CastToPlayerController (Pawn|GetController)))
  (Utilities|IsValid (PlayerController|LocalPlayerSubsystems|GetEnhancedInputLocalPlayerSubsystem _asplayer_controller)
    (:Is%20Valid
      (Input|AddMappingContext (PlayerController|LocalPlayerSubsystems|GetEnhancedInputLocalPlayerSubsystem _asplayer_controller) "/Game/Character/Actions/Inputs/IMC_Combat.IMC_Combat" 0 "(bIgnoreAllPressedKeysUntilRelease=True,bForceImmediately=False,bNotifyUserSettings=False)"))))

(fn ConstructionScript)

(fn FInterpWlakSpeed
  (Variables|/Script/Engine.CharacterMovementComponent|SetMaxWalkSpeed (Variables|Character|GetCharacterMovement) (Math|Interpolation|FInterpTo (Variables|/Script/Engine.CharacterMovementComponent|GetMaxWalkSpeed (Variables|Character|GetCharacterMovement)) (Variables|Default|GetWalkSpeed) (Utilities|Time|GetWorldDeltaSeconds) 0.5)))